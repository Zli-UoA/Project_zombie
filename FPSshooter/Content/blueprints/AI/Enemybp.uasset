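; Enemy actor Blueprint that can be killed for score and hurts the first-person player on contact.
; Incoming damage lowers a health variable (NewVar0); at zero or below it calls AddScore on the shootergamemode and destroys itself.
; A Damagepoint component applies a fixed damage amount to any FirstPersonCharacter that begins overlapping it.
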(event OnComponentBeginOverlap(damagepoint)
  (params (OverlappedComponent :type Primitive%20Component%20Object%20Reference) (OtherActor :type Actor%20Object%20Reference) (OtherComp :type Primitive%20Component%20Object%20Reference) (OtherBodyIndex :type Integer) (bFromSweep :type Boolean) (SweepResult :type Hit%20Result%20Structure%20%28by%20ref%29))
  (bind _asfirst_person_character (Utilities|Casting|CastToFirstPersonCharacter OtherActor))
  (Game|Damage|ApplyDamage _asfirst_person_character 1e+01 0 0))

(event Game|Damage|EventAnyDamage
  (params (Damage :type Float%20%28single-precision%29) (DamageType :type Damage%20Type%20Object%20Reference) (InstigatedBy :type Controller%20Object%20Reference) (DamageCauser :type Actor%20Object%20Reference))
  (bind _output_get (Variables|Default|SetNewVar_0 (- (Variables|Default|GetNewVar_0) Damage)))
  (if (<= _output_get 0.0)
    (bind _asshootergamemode (Utilities|Casting|CastToshootergamemode (Game|GetGameMode)))
    (Default|AddScore _asshootergamemode)
    (Actor|DestroyActor)))

(fn ConstructionScript)